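; BP_LammpsController starts and controls a LAMMPS particle simulation with in-game visualization.
; On BeginPlay it imports the LAMMPS DLL, then initializes the worker and particle visualization manager, optionally sets up dump-file animation playback over a timestep range, and applies the system scale.
; Left and right pause inputs both call Pause and print an on-screen message.
; Stat console commands and default particle-type setup are present but disconnected.
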(event EventBeginPlay
  (bind _returnvalue (Class|LammpsController|ImportLammps "LammpsDll" (Variables|Default|Getm_dllName)))
  (if _returnvalue
    (Class|LammpsController|InitializeWorkerandParticleVisualizationManager)
    ;[1 1 1] Animation Setup (if needed)
    (if (Variables|Default|Getm_animationMode)
      (Class|LammpsController|SetupAnimationState (Variables|Default|Getm_dumpFilePrefix) (Variables|Default|Getm_firstTimeStep) (Variables|Default|Getm_lastTimeStep) (Variables|Default|Getm_stepSize)))
    ;[1 1 1] Set System Scale
    (Class|LammpsController|SetSystemScale (Variables|Default|Getm_systemScale))))

(event Input|ActionEvents|InputActionPause_R
  (params (Key :type Key%20Structure :default "None"))
  (:Pressed
    (Class|LammpsController|Pause)
    (Development|PrintString "PAUSE" true true "(R=0.000000,G=0.660000,B=1.000000,A=1.000000)" 1e+06)))

(event Input|ActionEvents|InputActionPause_L
  (params (Key :type Key%20Structure :default "None"))
  (:Pressed
    (Class|LammpsController|Pause)
    (Development|PrintString "PAUSE" true true "(R=0.000000,G=0.660000,B=1.000000,A=1.000000)" 1e+06)))

(fn ConstructionScript)