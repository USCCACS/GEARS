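; BP_LammpsController starts a LAMMPS particle simulation and its in-game visualization.
; On BeginPlay it loads the LAMMPS DLL by name from the LammpsDll folder and continues only if the import succeeds.
; It then initializes the worker and particle visualization manager, registers colors and radii for three particle types, sets the system scale and synchronizes LAMMPS with the visualization manager.
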(event EventBeginPlay
  (bind _returnvalue (Class|LammpsController|ImportLammps "LammpsDll" (Variables|Default|Getm_dllName)))
  (if _returnvalue
    (Class|LammpsController|InitializeWorkerandParticleVisualizationManager)
    ;[1 1 1] Spawn New Particles Here
    (Class|LammpsController|ManageParticle 3 (Math|Conversions|ToColor(LinearColor) "(R=1.000000,G=0.000000,B=0.000000,A=1.000000)") 1.0)
    (Class|LammpsController|ManageParticle 4 (Math|Conversions|ToColor(LinearColor) "(R=1.000000,G=1.000000,B=0.000000,A=1.000000)") 1.11)
    (Class|LammpsController|ManageParticle 5 (Math|Conversions|ToColor(LinearColor) "(R=0.000000,G=0.380000,B=0.380000,A=1.000000)") 1.9)
    ;[1 1 1] Set System Scale
    (Class|LammpsController|SetSystemScale 2.5e+02)
    (Class|LammpsController|SynchronizeLammpsandParticleVisualizationManager)))

(event Collision|EventActorBeginOverlap
  (params (OtherActor :type Actor%20Object%20Reference)))

(event EventTick
  (params (DeltaSeconds :type Float%20%28single-precision%29)))

(fn ConstructionScript)